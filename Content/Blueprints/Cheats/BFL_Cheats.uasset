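; Cheat function library that adjusts two sensitivity variables on Character_YG by a given amount.
; BFLGOD casts player 0's character to Character_YG and adds the amount to Sensitiv1, printing an error if the cast fails.
; BFLTAR adds the amount to Sensitiv2 on a character passed in by the caller.
; Both functions print the resulting value to screen as feedback.
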(fn BFLGOD
  (params (B :type Float%20%28single-precision%29))
  (bind _ascharacter_yg (Utilities|Casting|CastToCharacter_YG (Game|GetPlayerCharacter 0))
    (:then
      (bind _output_get (Variables|/Game/Character/Character_YG.Character_YG_C|SetSensitiv1 _ascharacter_yg (+ (Variables|/Game/Character/Character_YG.Character_YG_C|GetSensitiv1 _ascharacter_yg) B)))
      (Development|PrintString 0 (Utilities|String|Append "Result of change " (Utilities|String|ToString(Float) _output_get))))
    (:CastFailed
      (Development|PrintString 0 "Character does not exist or other error"))))

(fn BFLTAR
  (params (Char :type Character%20YG%20Object%20Reference) (B :type Float%20%28single-precision%29))
  (bind _output_get (Variables|/Game/Character/Character_YG.Character_YG_C|SetSensitiv2 Char (+ (Variables|/Game/Character/Character_YG.Character_YG_C|GetSensitiv2 Char) B)))
  (Development|PrintString 0 (Utilities|String|Append "Result of change " (Utilities|String|ToString(Float) _output_get))))