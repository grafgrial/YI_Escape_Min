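; AC_Clock is an analog wall-style clock that animates second, minute and hour hand components from its own stored time, not the system clock.
; A looping one-second timer started on BeginPlay passes that time through SETActive, which increments it with rollover on a 12-hour cycle.
; The timer event then converts the result to pitch rotations, offsetting the hour hand by elapsed minutes for gradual movement.
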(event Custom|Timers
  (bind (_out_sec _out_min _out_hour) (CallFunction|SETActive (Variables|Default|GetSec) (Variables|Default|GetMin) (Variables|Default|GetHourss)))
  (Variables|Default|SetSec _out_sec)
  (Variables|Default|SetMin _out_min)
  (Variables|Default|SetHourss _out_hour)
  (Transformation|SetRelativeRotation (Variables|Default|GetClock02_SecondArrow) (Math|Rotator|MakeRotator 0.0 (* (Variables|Default|GetSec) -6.0) 0.0) false false)
  (Transformation|SetRelativeRotation (Variables|Default|GetClock02_MinutArrow) (Math|Rotator|MakeRotator 0.0 (* (Variables|Default|GetMin) -6.0) 0.0) false false)
  (Transformation|SetRelativeRotation (Variables|Default|GetClock02_HourArrow) (Math|Rotator|MakeRotator 0.0 (+ (* (Variables|Default|GetHourss) -3e+01) (* (/ (* (/ (* (Variables|Default|GetMin) 1e+02) 6e+01) 3e+01) 1e+02) -1.0)) 0.0) false false))

(event EventBeginPlay
  (|CallParentFunction)
  (bind _returnvalue (Utilities|Time|SetTimerbyEvent (delegate Custom|Timers) 1.0 true))
  (Variables|Default|SetClock_Timers _returnvalue))

(fn ConstructionScript
  (|CallParentFunction))

(fn SETActive
  (params (Inp_Second :type Integer) (Inp_Minute :type Integer) (Inp_Hour :type Integer))
  (Utilities|FlowControl|Sequence
    (:then_0
      (Utilities|FlowControl|DoOnce false
        (:Completed
          (LocalVariables|SetSecond Inp_Second)
          (LocalVariables|SetMinute Inp_Minute)
          (LocalVariables|SetHour Inp_Hour))))
    (:then_1
      (if (>= (+ (LocalVariables|GetSecond) 1) 60)
        (LocalVariables|SetSecond 0)
        (if (>= (+ (LocalVariables|GetMinute) 1) 60)
          (LocalVariables|SetMinute 0)
          (if (>= (+ (LocalVariables|GetHour) 1) 12)
            (LocalVariables|SetHour 0)
            (else
              (LocalVariables|SetHour (+ (LocalVariables|GetHour) 1))))
          (else
            (LocalVariables|SetMinute (+ (LocalVariables|GetMinute) 1))))
        (else
          (LocalVariables|SetSecond (+ (LocalVariables|GetSecond) 1))))
      (return (LocalVariables|GetSecond) (LocalVariables|GetMinute) (LocalVariables|GetHour)))))