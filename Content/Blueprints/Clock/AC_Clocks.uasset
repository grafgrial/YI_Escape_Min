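; Clock actor that animates second, minute and hour hands from its own time counter.
; A looping one-second timer started at BeginPlay passes the stored time through INTr, which adds a second and rolls over into minutes and a 12-hour count.
; The timer then sets each hand's relative pitch from the new values, offsetting the hour hand by the elapsed minutes so it moves gradually between hours.
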(event Custom|Timers
  (bind (_out_sec _out_min _out_hour) (CallFunction|INTr (Variables|Default|GetSec) (Variables|Default|GetMin) (Variables|Default|GetHourss)))
  (Variables|Default|SetSec _out_sec)
  (Variables|Default|SetMin _out_min)
  (Variables|Default|SetHourss _out_hour)
  (Transformation|SetRelativeRotation (Variables|Default|GetClock02_SecondArrow) (Math|Rotator|MakeRotator 0.0 (* (Variables|Default|GetSec) -6.0) 0.0) false false)
  (Transformation|SetRelativeRotation (Variables|Default|GetClock02_MinutArrow) (Math|Rotator|MakeRotator 0.0 (* (Variables|Default|GetMin) -6.0) 0.0) false false)
  (Transformation|SetRelativeRotation (Variables|Default|GetClock02_HourArrow) (Math|Rotator|MakeRotator 0.0 (+ (* (Variables|Default|GetHourss) -3e+01) (* (/ (* (/ (* (Variables|Default|GetMin) 1e+02) 6e+01) 3e+01) 1e+02) -1.0)) 0.0) false false))

(event EventBeginPlay
  (bind _returnvalue (Utilities|Time|SetTimerbyEvent (delegate Custom|Timers) 1.0 true))
  (Variables|Default|SetClock_Timers _returnvalue))

(fn ConstructionScript)

(fn INTr
  (params (Int_Second :type Integer) (Int_Minute :type Integer) (Int_Hour :type Integer))
  (Utilities|FlowControl|Sequence
    (:then_0
      (Utilities|FlowControl|DoOnce false
        (:Completed
          (LocalVariables|SetSecond Int_Second)
          (LocalVariables|SetMinute Int_Minute)
          (LocalVariables|SetHour Int_Hour))))
    (:then_1
      (if (>= (+ (LocalVariables|GetSecond) 1) 60)
        (LocalVariables|SetSecond 0)
        (if (>= (+ (LocalVariables|GetMinute) 1) 60)
          (LocalVariables|SetMinute 0)
          (if (>= (+ (LocalVariables|GetHour) 1) 12)
            (LocalVariables|SetHour 0)
            (else
              (LocalVariables|SetHour (+ (LocalVariables|GetHour) 1))))
          (else
            (LocalVariables|SetMinute (+ (LocalVariables|GetMinute) 1))))
        (else
          (LocalVariables|SetSecond (+ (LocalVariables|GetSecond) 1))))
      (return (LocalVariables|GetSecond) (LocalVariables|GetMinute) (LocalVariables|GetHour)))))