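; Interactable hinged door actor that swings open and closed when the player interacts with either of its two door components.
; Interaction runs a timeline forward or in reverse to lerp DoorCube's relative rotation, setting ISOpen from the direction when it finishes.
; Hover events toggle hovered feedback on the passed-in object.
; On BeginPlay it passes itself to GameInstance_YG's LoadActor.
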(event Custom|OpenDoor
  (if (Variables|Default|GetISOpen?)
    (bind (_direction _aplha) (Timeline|Timeline_0 Reverse)
      (:Update
        (Transformation|SetRelativeRotation (Variables|Default|GetDoor_Cube) (Math|Rotator|Lerp(Rotator) "0,0.000000, 0" "0,95.000000, 0" _aplha) false false))
      (:Finished
        (switch Utilities|FlowControl|Switch|SwitchonETimelineDirection _direction
          (:Forward
            (Variables|Default|SetISOpen? true))
          (:Backward
            (Variables|Default|SetISOpen? false)))))
    (else
      (Timeline|Timeline_0 Play))))

(event EventBeginPlay
  (bind _asgame_instance_yg (Utilities|Casting|CastToGameInstance_YG (Game|GetGameInstance)))
  (Default|LoadActor _asgame_instance_yg self))

(event EventActorHovered
  (params (NewParam :type Primitive%20Component%20Object%20Reference) (NewParam1 :type Character%20YG%20Object%20Reference))
  (if (or (== NewParam (Variables|Default|GetDoors)) (== NewParam (Variables|Default|GetDoors1)))
    (Default|WGHovered NewParam1)
    (else
      (Default|WGUnhovered NewParam1))))

(event EventActorInteract
  (params (Components :type Primitive%20Component%20Object%20Reference))
  (if (or (== Components (Variables|Default|GetDoors)) (== Components (Variables|Default|GetDoors1)))
    (CallFunction|OpenDoor)))

(fn ConstructionScript)