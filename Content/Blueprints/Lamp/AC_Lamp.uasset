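; AC_Lamp is a lamp actor whose spot light the player can switch on and off by interacting with it.
; An interact event on its Sphere component runs a FlipFlop that alternates the SpotLight intensity between lit and zero.
; A hover event on the same sphere calls WGHovered on the passed-in object, likely to show hover feedback.
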(event EventBeginPlay)

(event Collision|EventActorBeginOverlap
  (params (OtherActor :type Actor%20Object%20Reference)))

(event EventTick
  (params (DeltaSeconds :type Float%20%28single-precision%29)))

(event EventActorHovered
  (params (NewParam :type Primitive%20Component%20Object%20Reference) (NewParam1 :type Character%20YG%20Object%20Reference))
  (if (== NewParam (Variables|Default|GetSphere))
    (Default|WGHovered NewParam1)))

(event EventActorInteract
  (params (Components :type Primitive%20Component%20Object%20Reference))
  (bind _spotlight (Variables|Default|GetSpotLight))
  (if (== Components (Variables|Default|GetSphere))
    (Utilities|FlowControl|FlipFlop
      (:A
        (Rendering|Components|Light|SetIntensity _spotlight 5e+03))
      (:B
        (Rendering|Components|Light|SetIntensity _spotlight 0.0)))))

(fn ConstructionScript)