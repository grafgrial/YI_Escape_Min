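; Spawner that places target point actors showing random digits, apparently pieces of a four-digit code.
; On BeginPlay it rolls and prints four digits, then after a short delay spawns targets for only the first two, each at a random transform from its own position array.
; A macro looks up each digit in UVMat and splits the value into two material parameters on the target's plane, likely UV offsets selecting the digit.
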(event Custom|Spa
  (params (tag :type Array%20of%20Transforms) (Actor :type Actor%20Class%20Reference) (Count :type Integer))
  (bind _returnvalue (Game|SpawnActorfromClass Actor (Utilities|Array|Get(acopy) tag (Math|Random|RandomIntegerinRange 0 (Utilities|Array|LastIndex tag))) "Undefined" 0 0))
  (bind _asac_target_point (Utilities|Casting|CastToAC_TargetPoint _returnvalue))
  (bind (_newparam _newparam2) (Utilities|NewMacro0 Count)
    (:true
      (Rendering|Material|SetScalarParameterValueonMaterials (Variables|/Game/Blueprints/PointSpawn/AC_TargetPoint.AC_TargetPoint_C|GetPlane _asac_target_point) "Vpravo" _newparam)
      (Rendering|Material|SetScalarParameterValueonMaterials (Variables|/Game/Blueprints/PointSpawn/AC_TargetPoint.AC_TargetPoint_C|GetPlane _asac_target_point) "Vniz" _newparam2))))

(event EventBeginPlay
  (bind _returnvalue (Math|Random|RandomIntegerinRange 0 9))
  (bind _output_get (Variables|Default|Setcount_1 _returnvalue))
  (bind _output_get_2 (Variables|Default|Setcount_2 _returnvalue))
  (bind _output_get_3 (Variables|Default|Setcount_3 _returnvalue))
  (bind _output_get_4 (Variables|Default|Setcount_4 _returnvalue))
  (Development|PrintString (Utilities|String|Append (Utilities|String|ToString(Integer) _output_get) (Utilities|String|ToString(Integer) _output_get_2) (Utilities|String|ToString(Integer) _output_get_3) (Utilities|String|ToString(Integer) _output_get_4)))
  (Utilities|FlowControl|Delay 3.0)
  (CallFunction|Spa (Variables|Default|Gettag1Position) "/Game/Blueprints/PointSpawn/AC_TargetPoint.AC_TargetPoint_C" (Variables|Default|Getcount_1))
  (CallFunction|Spa (Variables|Default|Gettag2Position) "/Game/Blueprints/PointSpawn/AC_TargetPoint.AC_TargetPoint_C" (Variables|Default|Getcount_2)))

(fn ConstructionScript)