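; AC_Safe_Child is a child safe actor that responds to hover and interaction on a fixed set of its mesh components.
; BeginPlay runs the parent logic, then gathers a cylinder and three static meshes into an array that acts as the interactable whitelist.
; Hovering a listed component triggers the passed object's hovered widget state, otherwise the unhovered one.
; Interacting with a listed mesh swaps its first material slot to Mat_Stenki.
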(event EventBeginPlay
  (|CallParentFunction)
  (Variables|Default|SetCompon (Utilities|Array|MakeArray (Variables|Default|GetCylinder) (Variables|Default|GetStaticMesh1) (Variables|Default|GetStaticMesh2) (Variables|Default|GetStaticMesh3))))

(event Collision|EventActorBeginOverlap
  (params (OtherActor :type Actor%20Object%20Reference)))

(event EventTick
  (params (DeltaSeconds :type Float%20%28single-precision%29)))

(event EventActorHovered
  (params (NewParam :type Primitive%20Component%20Object%20Reference) (NewParam1 :type Character%20YG%20Object%20Reference))
  (if (>= (Utilities|Array|FindItem (Variables|Default|GetCompon) (.AsStatic%20Mesh%20Component (Utilities|Casting|CastToStaticMeshComponent NewParam))) 0)
    (Default|WGHovered NewParam1)
    (else
      (Default|WGUnhovered NewParam1))))

(event EventActorInteract
  (params (Components :type Primitive%20Component%20Object%20Reference))
  (bind _asstatic_mesh_component (Utilities|Casting|CastToStaticMeshComponent Components))
  (bind _compon (Variables|Default|GetCompon))
  (bind _returnvalue (Utilities|Array|FindItem _compon _asstatic_mesh_component))
  (if (>= _returnvalue 0)
    (Rendering|Material|SetMaterial (Utilities|Array|Get(acopy) _compon _returnvalue) 0 "/Game/Material/Mat_Stenki.Mat_Stenki")))

(fn ConstructionScript
  (|CallParentFunction))