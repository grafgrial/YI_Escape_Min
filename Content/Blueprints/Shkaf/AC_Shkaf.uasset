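; Interactable cabinet actor (shkaf) with three door meshes that swing open and closed when interacted with.
; Interaction maps the hit component to a door index, and that door's IsOpen flag picks forward or reverse play of one shared timeline.
; The timeline lerps the door to its per-index rotation, then stores and prints the open states.
; Hovering toggles the passed object's hover widget for valid doors, while interaction skips that validity check.
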(event Custom|OpenDoors
  (params (Target :type Scene%20Component%20Object%20Reference) (Dimension%201 :type Integer))
  (bind _isopen_ (Variables|Default|GetIsOpen?))
  (Utilities|NewMacro0 Dimension%201
    (:true
      (bind (_direction _alpha) (Timeline|Timeline_0 Reverse)
        (:Update
          (Transformation|SetRelativeRotation Target (Math|Rotator|Lerp(Rotator) "0,0.000000, 0" (Utilities|Array|Get(acopy) (Variables|Default|GetRotation) Dimension%201) _alpha) false false))
        (:Finished
          (switch Utilities|FlowControl|Switch|SwitchonETimelineDirection _direction
            (:Forward
              (Utilities|Array|SetArrayElem _isopen_ Dimension%201 true true))
            (:Backward
              (Utilities|Array|SetArrayElem _isopen_ Dimension%201 false true)))
          (for _array_element (Variables|Default|GetIsOpen?)
            (Development|PrintString (Utilities|String|ToString(Boolean) _array_element))))))
    (:false
      (Timeline|Timeline_0 Play))))

(event EventBeginPlay
  (Variables|Default|SetDooors (Utilities|Array|MakeArray (Variables|Default|GetShkaf_Cube_003) (Variables|Default|GetShkaf_Cube_0031) (Variables|Default|GetShkaf_Cube_002))))

(event EventActorInteract
  (params (Components :type Primitive%20Component%20Object%20Reference))
  (bind _asstatic_mesh_component (Utilities|Casting|CastToStaticMeshComponent Components))
  (bind _dooors (Variables|Default|GetDooors))
  (bind _returnvalue (Utilities|Array|FindItem _dooors _asstatic_mesh_component))
  (CallFunction|OpenDoors (Utilities|Array|Get(acopy) _dooors _returnvalue) _returnvalue))

(event EventActorHovered
  (params (NewParam :type Primitive%20Component%20Object%20Reference) (NewParam1 :type Character%20YG%20Object%20Reference))
  (bind _dooors (Variables|Default|GetDooors))
  (if (Utilities|Array|IsValidIndex _dooors (Utilities|Array|FindItem _dooors (.AsStatic%20Mesh%20Component (Utilities|Casting|CastToStaticMeshComponent NewParam))))
    (Default|WGHovered NewParam1)
    (else
      (Default|WGUnhovered NewParam1))))

(fn ConstructionScript)