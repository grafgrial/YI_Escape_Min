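; AC_Switch is an interactable switch that toggles a spotlight off and on.
; An ActorInteract event checks that the passed component is the Sphere, then a FlipFlop alternates the SpotLight intensity between zero and full brightness, switching it off on the first use.
; ActorHovered only prints a placeholder greeting, and the construction script just calls its parent.
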(event EventBeginPlay)

(event EventActorInteract
  (params (Components :type Primitive%20Component%20Object%20Reference))
  (bind _spotlight (Variables|Default|GetSpotLight))
  (if (== Components (Variables|Default|GetSphere))
    (Utilities|FlowControl|FlipFlop
      (:A
        (Rendering|Components|Light|SetIntensity _spotlight 0.0))
      (:B
        (Rendering|Components|Light|SetIntensity _spotlight 2.5e+04)))))

(event EventActorHovered
  (params (NewParam :type Primitive%20Component%20Object%20Reference))
  (Development|PrintString "Hello"))

(fn ConstructionScript
  (|CallParentFunction))