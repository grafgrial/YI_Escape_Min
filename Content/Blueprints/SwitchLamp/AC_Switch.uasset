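; AC_Switch is an interactable lamp switch that turns a spotlight off and on.
; An ActorInteract event on its Sphere component drives a FlipFlop, alternating the SpotLight intensity between zero and a bright value, starting with off.
; ActorHovered checks whether the hovered component is the Sphere and calls WGHovered or WGUnhovered on the passed-in object to update hover feedback.
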(event EventBeginPlay)

(event EventActorHovered
  (params (NewParam :type Primitive%20Component%20Object%20Reference) (NewParam1 :type Character%20YG%20Object%20Reference))
  (if (== NewParam (Variables|Default|GetSphere))
    (Default|WGHovered NewParam1)
    (else
      (Default|WGUnhovered NewParam1))))

(event EventActorInteract
  (params (Components :type Primitive%20Component%20Object%20Reference))
  (bind _spotlight (Variables|Default|GetSpotLight))
  (if (== Components (Variables|Default|GetSphere))
    (Utilities|FlowControl|FlipFlop
      (:A
        (Rendering|Components|Light|SetIntensity _spotlight 0.0))
      (:B
        (Rendering|Components|Light|SetIntensity _spotlight 2.5e+04)))))

(fn ConstructionScript
  (|CallParentFunction))