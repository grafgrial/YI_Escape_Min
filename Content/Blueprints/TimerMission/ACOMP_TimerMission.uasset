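; Mission countdown component that shows remaining hours, minutes and seconds in an on-screen WG_TimerMission widget.
; PlayTimer creates the widget and starts a looping one-second timer that calls TimerFunction.
; Each tick decrements Second, borrows from Minute and Hour, and pushes the unpadded H:M:S text to the widget.
; At zero it clears the timer, prints a debug string and removes the widget after TimeToDelWidget, with no mission-end event.
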(event EventBeginPlay)

(event EventTick
  (params (DeltaSeconds :type Float%20%28single-precision%29)))

(fn PlayTimer
  (bind _returnvalue (Utilities|Time|SetTimerbyFunctionName 0 "TimerFunction" 1.0 true))
  (Variables|Default|SetRef_TimerMission _returnvalue)
  (bind _returnvalue_2 (UserInterface|CreateWidget "/Game/Blueprints/TimerMission/WG_TimerMission.WG_TimerMission_C"))
  (bind _output_get (Variables|Default|SetRef_WG_TimerMission _returnvalue_2))
  (UserInterface|Viewport|AddtoViewport _output_get 0))

(fn TimerFunction
  (bind _result (Math|Integer|DecrementInt (Variables|Default|GetSecond))
    (:%20%20
      (CallFunction|WIdgettoText)
      (if (and (== (Math|Integer|Clamp(Integer) _result 0 59) 0) (> (Variables|Default|GetMinute) 0))
        (Variables|Default|SetSecond 59)
        (bind _result_2 (Math|Integer|DecrementInt (Variables|Default|GetMinute))
          (:%20%20
            (CallFunction|WIdgettoText)
            (if (and (== (Math|Integer|Clamp(Integer) _result_2 0 59) 0) (> (Variables|Default|GetHour) 0))
              (Variables|Default|SetMinute 59)
              (Math|Integer|DecrementInt (Variables|Default|GetHour)
                (:%20%20
                  _))))))
      (CallFunction|WIdgettoText)
      (if (Math|Boolean|ANDBoolean (== (Variables|Default|GetHour) 0) (== (Variables|Default|GetMinute) 0) (== (Variables|Default|GetSecond) 0))
        (CallFunction|WIdgettoText)
        (Development|PrintString "000000000")
        (CallFunction|TimerDelWidget)
        (Utilities|Time|ClearandInvalidateTimerbyHandle (Variables|Default|GetRef_TimerMission))))))

(fn TimerDelWidget
  (Utilities|Time|SetTimerbyFunctionName 0 "DelWidget" (Variables|Default|GetTimeToDelWidget)))

(fn DelWidget
  (bind _ref_wg_timermission (Variables|Default|GetRef_WG_TimerMission)
    (:then
      (Widget|RemovefromParent _ref_wg_timermission))
    (:else)))

(fn WIdgettoText
  (bind _ref_wg_timermission (Variables|Default|GetRef_WG_TimerMission)
    (:then
      (Rendering|Components|TextRender|SetText (Variables|/Game/Blueprints/TimerMission/WG_TimerMission.WG_TimerMission_C|GetText_timer _ref_wg_timermission) (Utilities|Text|ToText(String) (Utilities|String|Append (Utilities|String|ToString(Integer) (Variables|Default|GetHour)) ":" (Utilities|String|ToString(Integer) (Variables|Default|GetMinute)) ":" (Utilities|String|ToString(Integer) (Variables|Default|GetSecond))))))
    (:else)))