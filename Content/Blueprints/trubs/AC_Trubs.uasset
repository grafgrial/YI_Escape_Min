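; Actor with six clickable static meshes that the player rotates with the mouse, apparently pipe puzzle pieces.
; Box overlap by a player-instigated actor toggles player 0's mouse cursor and click events.
; Each mesh click runs a shared macro that, on left click, advances a yaw variable by 90 degrees, wrapping to zero, and applies it as relative rotation.
; A custom event casting Plane01's child to a box component leads to nothing further.
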(event OnComponentBeginOverlap(Box)
  (params (OverlappedComponent :type Primitive%20Component%20Object%20Reference) (OtherActor :type Actor%20Object%20Reference) (OtherComp :type Primitive%20Component%20Object%20Reference) (OtherBodyIndex :type Integer) (bFromSweep :type Boolean) (SweepResult :type Hit%20Result%20Structure%20%28by%20ref%29))
  (bind _returnvalue (Game|GetPlayerController 0))
  (if (Pawn|IsPlayerControlled (Variables|/Script/Engine.Actor|GetInstigator OtherActor))
    (Variables|/Script/Engine.PlayerController|SetbShowMouseCursor _returnvalue true)
    (Variables|/Script/Engine.PlayerController|SetbEnableClickEvents _returnvalue true)))

(event OnClicked(StaticMesh)
  (params (TouchedComponent :type Primitive%20Component%20Object%20Reference) (ButtonPressed :type Key%20Structure :default "AnyKey"))
  (Utilities|NewMacro0 (Variables|Default|GetStaticMesh) ButtonPressed))

(event OnClicked(StaticMesh1)
  (params (TouchedComponent :type Primitive%20Component%20Object%20Reference) (ButtonPressed :type Key%20Structure :default "AnyKey"))
  (Utilities|NewMacro0 (Variables|Default|GetStaticMesh1) ButtonPressed))

(event OnClicked(StaticMesh2)
  (params (TouchedComponent :type Primitive%20Component%20Object%20Reference) (ButtonPressed :type Key%20Structure :default "AnyKey"))
  (Utilities|NewMacro0 (Variables|Default|GetStaticMesh2) ButtonPressed))

(event OnClicked(StaticMesh3)
  (params (TouchedComponent :type Primitive%20Component%20Object%20Reference) (ButtonPressed :type Key%20Structure :default "AnyKey"))
  (Utilities|NewMacro0 (Variables|Default|GetStaticMesh3) ButtonPressed))

(event OnClicked(StaticMesh4)
  (params (TouchedComponent :type Primitive%20Component%20Object%20Reference) (ButtonPressed :type Key%20Structure :default "AnyKey"))
  (Utilities|NewMacro0 (Variables|Default|GetStaticMesh4) ButtonPressed))

(event OnClicked(StaticMesh5)
  (params (TouchedComponent :type Primitive%20Component%20Object%20Reference) (ButtonPressed :type Key%20Structure :default "AnyKey"))
  (Utilities|NewMacro0 (Variables|Default|GetStaticMesh5) ButtonPressed))

(event OnComponentEndOverlap(Box)
  (params (OverlappedComponent :type Primitive%20Component%20Object%20Reference) (OtherActor :type Actor%20Object%20Reference) (OtherComp :type Primitive%20Component%20Object%20Reference) (OtherBodyIndex :type Integer))
  (bind _returnvalue (Game|GetPlayerController 0))
  (if (Pawn|IsPlayerControlled (Variables|/Script/Engine.Actor|GetInstigator OtherActor))
    (Variables|/Script/Engine.PlayerController|SetbShowMouseCursor _returnvalue false)
    (Variables|/Script/Engine.PlayerController|SetbEnableClickEvents _returnvalue false)))

(event Custom|CustomEvent_0
  (bind _asbox_collision (Utilities|Casting|CastToBoxComponent (Components|GetChildComponent (Variables|Default|Getplane01) 0))))

(event EventBeginPlay)

(event Collision|EventActorBeginOverlap
  (params (OtherActor :type Actor%20Object%20Reference)))

(event EventTick
  (params (DeltaSeconds :type Float%20%28single-precision%29)))

(fn ConstructionScript)